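; Server-authoritative destruction objective area that spawns a weapon cache at a random tagged spawn location and reports the objective met when it is destroyed.
; With UseFakeMarkers, it picks random spots a minimum distance apart, placing the cache at one and markers at all; otherwise, one approximate marker is used.
; Discovering the real marker clears the fakes; discovering the last fake force-reveals the real one.
; BP_MapPainter_V2 draws the area border until destruction.
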(event Custom|MarkerDiscovered
  (params (Discovered%20Marker :type Actor%20Object%20Reference) (is%20Real%20Cache :type Boolean))
  (bind _possiblespotsmarkers (Variables|Default|GetPossibleSpotsMarkers))
  ;[1 1 1] Handling event of marker discovering (triggers when player comes close to marker position)
  (Networking|SwitchHasAuthority
    (:Authority
      (if is%20Real%20Cache ; if marker was "real"
        (for _array_element (Variables|Default|GetPossibleSpotsMarkers)
          (Actor|DestroyActor _array_element) ; Destroy all "fake" markers
        )
        (Utilities|Array|Clear (Variables|Default|GetPossibleSpotsMarkers))
        (else
          (Utilities|Array|RemoveItem _possiblespotsmarkers Discovered%20Marker) ; if marker was "fake", remove it from list
          (Actor|DestroyActor Discovered%20Marker) ; and destroy
          (if (not (> (Utilities|Array|Length _possiblespotsmarkers) 0)) ; if it was last "fake" marker left
            (bind _asbp_destruction_attack_marker (Utilities|Casting|CastToBP_Destruction_AttackMarker (Variables|Default|GetCache%20Marker)))
            (Default|ForceDiscoverasLastMarker _asbp_destruction_attack_marker) ; then force set "real" marker as discovered
          ))))))

(event Custom|OnCacheDestroyed
  (params (Objective :type SQ%20Objective%20Object%20Reference))
  ;[1 1 1] Handling event of weapon cache destruction
  (Networking|SwitchHasAuthority
    (:Authority
      (Development|PrintString "Objective met, notifying PhaseDirector")
      (Class|SQObjective|SetObjectiveMet true "Team_Two")
      (Default|CallDestructionObjectiveMet self)
      (Utilities|IsValid (Variables|Default|GetCache%20Marker)
        (:Is%20Valid
          (Actor|DestroyActor (Variables|Default|GetCache%20Marker))
          (Variables|Default|SetCache%20Marker 0))
        (:Is%20Not%20Valid
          _))
      ;[1 1 1] Handling of border area spline painting on map
      (bind _outactors (Actor|GetAllActorsOfClass "/Chora_DES_v1/Gameplay/MapPaint/BP_MapPainter_V2.BP_MapPainter_V2_C"))
      (Utilities|IsValid (Utilities|Array|Get(acopy) _outactors)
        (:Is%20Valid
          (Default|RemoveDrawedSpline (Utilities|Array|Get(acopy) _outactors) (Variables|Gameplay|GetObjectiveAreaBorder)))))))

(event Custom|OnShown
  (params (Objective%20class :type SQ%20Objective%20Class%20Reference))
  (bind _returnvalue (Transformation|GetActorTransform))
  (bind _randomsource (Variables|Default|GetRandomSource))
  (Networking|SwitchHasAuthority
    (:Authority
      (if (Variables|Gameplay|GetUseFakeMarkers)
        ;[1 1 1] Picking set of spawn spots, dispersed by minimum distance, spawn cache on random spot from that set
        (bind _picked_dispersed_spots (CallFunction|PickRandomSpots (Variables|Default|GetCache%20spawn%20spots) (Variables|Gameplay|GetNumber%20of%20spots) (Variables|Gameplay|GetMin%20Distance%20Between%20Spots) _randomsource)) ; Pick set amount of random spots from array, with minimum distance between eachother
        (bind _output_get (Variables|Default|SetReal%20Spot (.Element (Utilities|PickRandomArrayElement _picked_dispersed_spots _randomsource))))
        (bind _returnvalue_2 (Game|SpawnActorfromClass Objective%20class (Transformation|GetActorTransform _output_get) "Undefined" self 0)) ; Spawn cache on random spot from the list of picked dispersed spots
        (Variables|Default|SetCurrent%20Cache _returnvalue_2)
        (else
          ;[1 0.29 0.29] Spawning cache on random spot from list (OLD SYSTEM)
          (bind _returnvalue_3 (Game|SpawnActorfromClass Objective%20class (Transformation|GetActorTransform (.Element (Utilities|PickRandomArrayElement (Variables|Default|GetCache%20spawn%20spots) (Variables|Default|GetRandomSource)))) "Undefined" self 0))
          ;[1 1 1] Configuring spawned cache, binding handler for cache destruction event
          (bind _output_get_2 (Variables|Default|SetCurrent%20Cache _returnvalue_3))))
      (Class|SQTeamActor|SetTeam _output_get_2 (Variables|Default|GetTeam))
      (bind _asbp_destruction_cache (Utilities|Casting|CastToBP_DestructionCache _output_get_2))
      (EventDispatchers|BindEventtoOnCacheDestroyed _asbp_destruction_cache (delegate Custom|OnCacheDestroyed))
      (Default|Show _asbp_destruction_cache)
      (Utilities|IsValid (Variables|Gameplay|GetObjectiveAreaBorder)
        (:Is%20Valid
          ;[1 1 1] Handling of border area spline painting on map
          (bind _outactors (Actor|GetAllActorsOfClass "/Chora_DES_v1/Gameplay/MapPaint/BP_MapPainter_V2.BP_MapPainter_V2_C"))
          (Utilities|IsValid (Utilities|Array|Get(acopy) _outactors)
            (:Is%20Valid
              (Default|AddDrawedSpline (Utilities|Array|Get(acopy) _outactors) (Variables|Gameplay|GetObjectiveAreaBorder)))))
        (:Is%20Not%20Valid
          _))
      (if (Variables|Gameplay|GetUseFakeMarkers)
        ;[1 1 1] Spawning markers on all spots from dispersed spots set, setting them as "fake" or "real", binding handler for event of discovering marker area
        (for _array_element _picked_dispersed_spots ; For each of picked dispersed spots
          (bind _returnvalue_4 (Game|SpawnActorfromClass "/Chora_DES_v1/Gameplay/BP_Destruction_AttackMarker.BP_Destruction_AttackMarker_C" (Transformation|GetActorTransform _array_element) "Undefined" self (== _array_element (Variables|Default|GetReal%20Spot)) 0)) ; Spawn possible cache spot marker
          (if (== _array_element (Variables|Default|GetReal%20Spot))
            (Variables|Default|SetCache%20Marker _returnvalue_4) ; Save a reference to "real" spot marker
          )
          (Class|SQTeamActor|SetTeam _returnvalue_4 (CallFunction|GetOpposingTeam))
          (Class|SQMapMarker|SetMarkerVisibleto _returnvalue_4 "Team")
          (EventDispatchers|BindEventtoDiscovered _returnvalue_4 (delegate Custom|MarkerDiscovered))
          (if (not (== _array_element (Variables|Default|GetReal%20Spot))) ; Only add "fake" markers into array
            (Utilities|Array|Add (Variables|Default|GetPossibleSpotsMarkers) _returnvalue_4)))
        (else
          ;[1 0.37 0.37] Spawn and configure single, not-exact position marker (OLD SYSTEM)
          (bind _returnvalue_5 (Game|SpawnActorfromClass "/Game/Gameplay/GameModes/BP_Insurgency_KnownAttackMarker.BP_Insurgency_KnownAttackMarker_C" (Math|Transform|MakeTransform (+ (.location _returnvalue) "0, 0,100.000000") (.rotation _returnvalue) "1,1,1") "Undefined" self 0))
          (Class|SQTeamActor|SetTeam _returnvalue_5 (CallFunction|GetOpposingTeam))
          (Class|SQMapMarker|SetMarkerVisibleto _returnvalue_5 "Team")
          (Variables|Default|SetCache%20Marker _returnvalue_5))))))

(event EventBeginPlay
  ;[1 0.8883 0.7515] Initialization of objective
  (Networking|SwitchHasAuthority
    (:Authority
      (Class|KismetMathLibrary|SeedRandomStream (Variables|Default|GetRandomSource))
      (bind _outactors (Actor|GetAllActorswithTag (Variables|Gameplay|GetObjectiveTag))) ; Finding all caches with same tag
      (for _array_element _outactors
        (bind _asbp_objective_spawn_location (Utilities|Casting|CastToBP_ObjectiveSpawnLocation _array_element))
        (Utilities|Array|Add (Variables|Default|GetCache%20spawn%20spots) _asbp_objective_spawn_location)))))

(event Collision|EventActorBeginOverlap
  (params (OtherActor :type Actor%20Object%20Reference)))

(event EventTick
  (params (DeltaSeconds :type Float%20%28single-precision%29)))

(fn ConstructionScript)

(fn GetCache
  (return (Variables|Default|GetCurrent%20Cache)))

(fn PickRandomSpots
  (params (Spots%20list :type Array%20of%20Actor%20Object%20References) (Number%20of%20spots :type Integer) (Dispersion :type Float%20%28single-precision%29) (Rand%20Source :type Random%20Stream%20Structure))
  (bind _non_matched_list (LocalVariables|GetNon-Matched%20list))
  (bind _result_list (LocalVariables|GetResult%20List))
  (Utilities|FlowControl|Sequence
    (:then_0
      (LocalVariables|SetInitial%20List Spots%20list)
      (LocalVariables|SetAmount Number%20of%20spots)
      (LocalVariables|SetDispersion%20Distance Dispersion)
      (LocalVariables|SetRand Rand%20Source))
    (:then_1
      (Utilities|Array|Clear (LocalVariables|GetResult%20List))
      (Utilities|MoveItemfromArray (LocalVariables|GetResult%20List) (LocalVariables|GetInitial%20List) (.Index (Utilities|PickRandomArrayElement (LocalVariables|GetInitial%20List) (LocalVariables|GetRand)))
        (:Output
          (while (and (< (Utilities|Array|Length (LocalVariables|GetResult%20List)) (LocalVariables|GetAmount)) (not (LocalVariables|GetLoop%20Break)))
            (LocalVariables|SetMatch-test%20list (LocalVariables|GetInitial%20List)) ; Copy leftovers into test list
            (bind _array_element (Utilities|Array|ForEachLoopwithBreak (LocalVariables|GetResult%20List) :!label _label) ; For each result list element
              (:LoopBody
                (if (> (Utilities|Array|Length (LocalVariables|GetMatch-test%20list)) 0) ; stop if test list is empty
                  (for _array_element_2 (LocalVariables|GetMatch-test%20list) ; check each test list element
                    (if (< (Transformation|GetHorizontalDistanceTo _array_element _array_element_2) (LocalVariables|GetDispersion%20Distance)) ; If it is too close to current result list element
                      (Utilities|Array|Add (LocalVariables|GetNon-Matched%20list) _array_element_2) ; then add it to non-matched list
                    ))
                  (Utilities|DeleteArrayfromArray (LocalVariables|GetMatch-test%20list) _non_matched_list ; Delete non-matched from test list
                    (:Out
                      (Utilities|Array|Clear _non_matched_list) ; clear non-matched list
                    ))
                  (else
                    (LocalVariables|SetLoop%20Break true)
                    (goto _label Break))))
              (:Completed
                (if (> (Utilities|Array|Length (LocalVariables|GetMatch-test%20list)) 0) ; After all checks passed
                  (Utilities|MoveItemfromArray (LocalVariables|GetResult%20List) (LocalVariables|GetInitial%20List) (Utilities|Array|FindItem (LocalVariables|GetInitial%20List) (.Element (Utilities|PickRandomArrayElement (LocalVariables|GetMatch-test%20list) (LocalVariables|GetRand))))) ; Move it from initial list to result list
                  (else
                    (LocalVariables|SetLoop%20Break true) ; stop if test list is empty
                  )))))
          (for _array_element_3 _result_list
            (Rendering|Debug|DrawDebugSphere (Transformation|GetActorLocation _array_element_3) 1e+02 12 "(R=1.000000,G=0.029832,B=0.000000,A=1.000000)" 1e+01))
          (return _result_list))))))

(fn GetOpposingTeam
  (switch Utilities|FlowControl|Switch|SwitchonESQTeam (Class|SQTeamActor|GetTeam)
    (:Team_Neutral
      (return "Team_Neutral"))
    (:Team_One
      (return "Team_Two"))
    (:Team_Two
      (return "Team_One"))))