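; No-deploy zone actor that removes itself when the destruction phase director starts its configured removal phase.
; On authority, BeginPlay binds to the director's phase event after a delay, retrying until one is found.
; Border events act only on the remote side, adding or removing the AreaBorder spline on the map painter.
; Both border drawing and zone destruction require a valid AreaBorder.
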(event Custom|Phase%20Start
  (params (Phase%20Number :type Integer))
  (Networking|SwitchHasAuthority
    (:Authority
      (if (== Phase%20Number (Variables|Default|GetRemove%20on%20phase))
        (Development|PrintString "Removing NoDeployZone" true true "(R=0.000000,G=0.660000,B=1.000000,A=1.000000)" 5.0)
        (Utilities|IsValid (Variables|Default|GetAreaBorder)
          (:Is%20Valid
            (CallFunction|RemoveBorderonClient)
            (Actor|DestroyActor)))))))

(event Custom|Retry%20Init
  (Networking|SwitchHasAuthority
    (:Authority
      (Utilities|FlowControl|Delay 2.0)
      (bind _outactors (Actor|GetAllActorsOfClass "/Chora_DES_v1/Gameplay/BP_DestructionPhaseDirector.BP_DestructionPhaseDirector_C"))
      (Utilities|IsValid (Utilities|Array|Get(acopy) _outactors)
        (:Is%20Valid
          (EventDispatchers|BindEventtoPhaseStarted (Utilities|Array|Get(acopy) _outactors) (delegate Custom|Phase%20Start))
          (Utilities|IsValid (Variables|Default|GetAreaBorder)
            (:Is%20Valid
              (CallFunction|AddBorderonClient))))
        (:Is%20Not%20Valid
          (Development|PrintString "Phase Director actor not found!" true true "(R=1.000000,G=0.000000,B=0.016322,A=1.000000)")
          (CallFunction|RetryInit))))))

(event Custom|AddBorderOnClient
  (Networking|SwitchHasAuthority
    (:Remote
      (bind _outactors (Actor|GetAllActorsOfClass "/Chora_DES_v1/Gameplay/MapPaint/BP_MapPainter_V2.BP_MapPainter_V2_C"))
      (Utilities|IsValid (Utilities|Array|Get(acopy) _outactors)
        (:Is%20Valid
          (Default|AddDrawedSpline (Utilities|Array|Get(acopy) _outactors) (Variables|Default|GetAreaBorder)))))))

(event Custom|RemoveBorderOnClient
  (Networking|SwitchHasAuthority
    (:Remote
      (bind _outactors (Actor|GetAllActorsOfClass "/Chora_DES_v1/Gameplay/MapPaint/BP_MapPainter_V2.BP_MapPainter_V2_C"))
      (Utilities|IsValid (Utilities|Array|Get(acopy) _outactors)
        (:Is%20Valid
          (Default|RemoveDrawedSpline (Utilities|Array|Get(acopy) _outactors) (Variables|Default|GetAreaBorder)))))))

(event EventBeginPlay
  (Networking|SwitchHasAuthority
    (:Authority
      (Utilities|FlowControl|Delay 2.0)
      (bind _outactors (Actor|GetAllActorsOfClass "/Chora_DES_v1/Gameplay/BP_DestructionPhaseDirector.BP_DestructionPhaseDirector_C"))
      (Utilities|IsValid (Utilities|Array|Get(acopy) _outactors)
        (:Is%20Valid
          (EventDispatchers|BindEventtoPhaseStarted (Utilities|Array|Get(acopy) _outactors) (delegate Custom|Phase%20Start))
          (Utilities|IsValid (Variables|Default|GetAreaBorder)
            (:Is%20Valid
              (CallFunction|AddBorderonClient))))
        (:Is%20Not%20Valid
          (Development|PrintString "Phase Director actor not found!" true true "(R=1.000000,G=0.000000,B=0.016322,A=1.000000)")
          (CallFunction|RetryInit))))))

(fn ConstructionScript)