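; BP_Destruction_TempSpawn creates a temporary team spawn point at its own location for a phase of the Destruction game mode.
; After a short startup delay, the server binds to the phase director's phase start or end event per ActivateOnPhaseStart, destroying itself if none is found.
; On a matching phase number, it spawns an SQGameSpawn for the team opposing the last phase's winner, limited by Lifetime.
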(event Custom|Event%20Activate
  (params (Phase%20Number :type Integer))
  (Networking|SwitchHasAuthority
    (:Authority
      (if (== Phase%20Number (Variables|Behaviour|GetPhase%20Number))
        (bind _returnvalue (Game|SpawnActorfromClass "/Script/Squad.SQGameSpawn" (Transformation|GetActorTransform) "Undefined" self 0))
        (bind _output_get (Variables|Components|SetSpawnPoint _returnvalue))
        (switch Utilities|FlowControl|Switch|SwitchonESQTeam (Variables|/Chora_DES_v1/Gameplay/BP_DestructionPhaseDirector.BP_DestructionPhaseDirector_C|GetWinningTeamOnLastPhaseComplete (Utilities|Array|Get(acopy) (stale EventBeginPlay _outactors)))
          (:Team_One
            (Class|SQGameSpawn|SetTeam _output_get "Team_Two"))
          (:Team_Two
            (Class|SQGameSpawn|SetTeam _output_get "Team_One")))
        (Actor|SetLifeSpan _output_get (Variables|Behaviour|GetLifetime))))))

(event EventBeginPlay
  (Utilities|FlowControl|Delay 3.0)
  (Networking|SwitchHasAuthority
    (:Authority
      (bind _outactors (Actor|GetAllActorsOfClass "/Chora_DES_v1/Gameplay/BP_DestructionPhaseDirector.BP_DestructionPhaseDirector_C"))
      (Utilities|IsValid (Utilities|Array|Get(acopy) _outactors)
        (:Is%20Valid
          (if (Variables|Behaviour|GetActivate%20on%20phase%20start)
            (EventDispatchers|BindEventtoPhaseStarted (Utilities|Array|Get(acopy) _outactors) (EventDispatchers|CreateEvent :!event Custom|Event%20Activate))
            (else
              (EventDispatchers|BindEventtoPhaseEnded (Utilities|Array|Get(acopy) _outactors) (EventDispatchers|CreateEvent :!event Custom|Event%20Activate)))))
        (:Is%20Not%20Valid
          (Development|PrintString "TempSpawn: No phase director found" true true "(R=0.000000,G=0.660000,B=1.000000,A=1.000000)" 5.0)
          (Actor|DestroyActor))))))

(event EventTick
  (params (DeltaSeconds :type Float%20%28single-precision%29)))

(fn ConstructionScript)