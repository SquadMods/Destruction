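; Destructible Insurgency cache objective that explodes with radial damage and swaps to a destroyed mesh, briefly toggling mobility to do so.
; The server sizes a child-actor no-deploy zone and spawns a team-visible defend marker on Show.
; When met, it notifies the objective actor and removes marker and zone.
; Thermite damage triggers separate radial damage, and team 1 players get a line-of-sight text prompt until completion.
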(event Custom|Show
  (bind _returnvalue (Transformation|GetActorTransform))
  (Networking|SwitchHasAuthority
    (:Authority
      (bind _returnvalue_2 (Game|SpawnActorfromClass "/Game/Gameplay/GameModes/BP_Insurgency_KnownDefendMarker.BP_Insurgency_KnownDefendMarker_C" (Math|Transform|MakeTransform (+ (.location _returnvalue) "0, 0,100.000000") (.rotation _returnvalue) "1,1,1") "Undefined" self 0))
      (Variables|Default|SetMarker _returnvalue_2)
      (Class|SQMapMarker|SetMarkerVisibleto _returnvalue_2 "Team")
      (Class|SQTeamActor|SetTeam _returnvalue_2 (Class|SQTeamActor|GetTeam)))))

(event EventOnMet
  (Networking|SwitchHasAuthority
    (:Authority
      (Development|PrintString "Cache died, notifying objective actor")
      (Default|CallOnCacheDestroyed self)
      (Actor|DestroyActor (Variables|Default|GetMarker))
      (Variables|Default|SetMarker 0)
      (Networking|SwitchHasAuthority
        (:Authority
          (bind _asbp_no_deploy_zone (Utilities|Casting|CastToBP_NoDeployZone (Variables|/Script/Engine.ChildActorComponent|GetChildActor (Variables|Default|GetCacheNoDeployZone))))
          (Components|Sphere|SetSphereRadius (Variables|/Game/Blueprints/Placeable/BP_NoDeployZone.BP_NoDeployZone_C|GetSphereCollision _asbp_no_deploy_zone) 1.0 true)
          (Components|DestroyComponent (Variables|Default|GetCacheNoDeployZone)))))))

(event EventBPHidePrompt
  (bind _return_value (CallFunction|GetSquadPlayerController))
  (if (Variables|Default|GetbHasObjectiveBeenMet)
    (Utilities|FlowControl|DoOnce false
      (:Completed
        _)))
  (if (Utilities|IsValid _return_value)
    (bind _assqplayer_state (Utilities|Casting|CastToSQPlayerState (Variables|/Script/Engine.Controller|GetPlayerState _return_value)))
    (Utilities|Array|RemoveItem (Variables|/Script/Squad.SQPlayerState|GetLineOfSightDrawTextCache _assqplayer_state) self)))

(event Game|Damage|EventAnyDamage
  (params (Damage :type Float%20%28single-precision%29) (DamageType :type Damage%20Type%20Object%20Reference) (InstigatedBy :type Controller%20Object%20Reference) (DamageCauser :type Actor%20Object%20Reference))
  (Utilities|Casting|CastToSQDamageType_Thermite DamageType)
  (Class|GameplayStatics|ApplyRadialDamagewithFalloff (Variables|DamageTakenExplosion|GetAnyDamageBaseDamage) (Variables|DamageTakenExplosion|GetAnyDamageMinimumDamage) (Transformation|GetActorLocation) (Variables|DamageTakenExplosion|GetAnyDamageInnerRadius) (Variables|DamageTakenExplosion|GetAnyDamageOuterRadius) (Variables|DamageTakenExplosion|GetAnyDamageDamageFalloff) "/Engine/EngineDamageTypes/DmgTypeBP_Environmental.DmgTypeBP_Environmental_C" 0 self (Game|GetInstigatorController) "ECC_WorldStatic"))

(event EventBPDisplayPrompt
  (params (User :type Controller%20Object%20Reference))
  (if (not (Variables|Default|GetbHasObjectiveBeenMet))
    (bind _assqplayer_state (Utilities|Casting|CastToSQPlayerState (Variables|/Script/Engine.Controller|GetPlayerState User)))
    (if (and (Utilities|IsValid (Variables|/Script/Squad.SQPlayerState|GetTeamState _assqplayer_state)) (== (Variables|/Script/Squad.SQTeamState|GetId (Variables|/Script/Squad.SQPlayerState|GetTeamState _assqplayer_state)) 1))
      (Utilities|Array|AddUnique (Variables|/Script/Squad.SQPlayerState|GetLineOfSightDrawTextCache _assqplayer_state) self))))

(event EventBPClientObjectiveDestroyed
  (bind _staticmesh (Variables|Default|GetStaticMesh))
  (Class|SQBlueprintLibrary|SetMobility _staticmesh "Stationary")
  (Components|StaticMesh|SetStaticMesh _staticmesh (Variables|Objective|GetDestroyedMesh))
  (Class|SQBlueprintLibrary|SetMobility _staticmesh "Static")
  (Class|GameplayStatics|ApplyRadialDamagewithFalloff (Variables|ObjectiveDestroyable|GetExplosionBaseDamage) (Variables|ObjectiveDestroyable|GetExplosionMinimumDamage) (+ (Transformation|GetActorLocation) "0, 0,50.000000") (Variables|ObjectiveDestroyable|GetExplosionDamageInnerRadius) (Variables|ObjectiveDestroyable|GetExplosionDamageOuterRadius) (Variables|ObjectiveDestroyable|GetExplosionDamageFalloff) "/Engine/EngineDamageTypes/DmgTypeBP_Environmental.DmgTypeBP_Environmental_C" 0 self (Game|GetInstigatorController) "ECC_WorldStatic"))

(event EventObjectiveDestroyed
  (params (Damage :type Float%20%28single-precision%29) (DamageEvent :type Damage%20Event%20Structure%20%28by%20ref%29) (EventInstigator :type Controller%20Object%20Reference) (DamageCauser :type Actor%20Object%20Reference))
  (bind _staticmesh (Variables|Default|GetStaticMesh))
  (Class|SQBlueprintLibrary|SetMobility _staticmesh "Stationary")
  (Components|StaticMesh|SetStaticMesh _staticmesh (Variables|Objective|GetDestroyedMesh))
  (Class|SQBlueprintLibrary|SetMobility _staticmesh "Static")
  (Class|GameplayStatics|ApplyRadialDamagewithFalloff (Variables|ObjectiveDestroyable|GetExplosionBaseDamage) (Variables|ObjectiveDestroyable|GetExplosionMinimumDamage) (+ (Transformation|GetActorLocation) "0, 0,50.000000") (Variables|ObjectiveDestroyable|GetExplosionDamageInnerRadius) (Variables|ObjectiveDestroyable|GetExplosionDamageOuterRadius) (Variables|ObjectiveDestroyable|GetExplosionDamageFalloff) "/Engine/EngineDamageTypes/DmgTypeBP_Environmental.DmgTypeBP_Environmental_C" 0 self (Game|GetInstigatorController) "ECC_WorldStatic"))

(event EventBeginPlay
  (Networking|SwitchHasAuthority
    (:Authority
      (bind _asbp_no_deploy_zone (Utilities|Casting|CastToBP_NoDeployZone (Variables|/Script/Engine.ChildActorComponent|GetChildActor (Variables|Default|GetCacheNoDeployZone))))
      (Components|Sphere|SetSphereRadius (Variables|/Game/Blueprints/Placeable/BP_NoDeployZone.BP_NoDeployZone_C|GetSphereCollision _asbp_no_deploy_zone) 1e+03 true))))

(fn ConstructionScript
  (bind _staticmesh (Variables|Default|GetStaticMesh))
  (Components|StaticMesh|SetStaticMesh _staticmesh (Variables|Objective|GetActiveMesh))
  (Class|SQBlueprintLibrary|SetMobility _staticmesh "Static"))