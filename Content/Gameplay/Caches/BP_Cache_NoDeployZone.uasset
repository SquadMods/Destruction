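; BP_Cache_NoDeployZone is a sphere volume for caches, named as a zone where deployment is disallowed.
; The construction script sizes the collision sphere from the SphereRadius variable.
; EnableCollisions and DisableCollisions events switch the sphere between query-only collision with overlap events and no collision without them.
; The Blueprint holds no overlap or deploy-blocking logic of its own.
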(event Custom|DisableCollisions
  (bind _spherecollision (Variables|Default|GetSphereCollision))
  (Collision|SetCollisionEnabled _spherecollision "NoCollision")
  (Variables|/Script/Engine.PrimitiveComponent|SetbGenerateOverlapEvents _spherecollision false))

(event Custom|EnableCollisions
  (bind _spherecollision (Variables|Default|GetSphereCollision))
  (Collision|SetCollisionEnabled _spherecollision "QueryOnly")
  (Variables|/Script/Engine.PrimitiveComponent|SetbGenerateOverlapEvents _spherecollision true))

(event EventBeginPlay)

(event Collision|EventActorBeginOverlap
  (params (OtherActor :type Actor%20Object%20Reference)))

(event EventTick
  (params (DeltaSeconds :type Float%20%28single-precision%29)))

(fn ConstructionScript
  (Components|Sphere|SetSphereRadius (Variables|Default|GetSphereCollision) (Variables|Default|GetSphereRadius) true))