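; Directs a phased Destruction game mode in which attackers clear successive sets of objectives owned by the opposing team.
; The server binds and reveals each phase's objectives, adjusts tickets on completion, and ends the last phase or schedules the next.
; A looping timer tells attackers the time until new orders.
; Clients draw a map lattice of splines linking objectives to phase centroids and consecutive centroids, via BP_MapPainter_V2.
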(event Custom|Event%20StartNewPhase
  (bind _updatetimer (Variables|Default|GetUpdateTimer))
  (Utilities|Time|PauseTimerbyHandle _updatetimer)
  (Utilities|Time|ClearandInvalidateTimerbyHandle _updatetimer)
  (Utilities|Time|ClearandInvalidateTimerbyHandle (Variables|Default|GetPhaseStartTimer))
  (Development|PrintString (Utilities|String|Append "Starting phase " (Utilities|String|ToString(Integer) (+ (Variables|Gameplay|GetCurrentPhase) 1)) " out of " (Utilities|String|ToString(Integer) (Variables|Gameplay|GetNumberOfPhases))) true true "(R=0.000000,G=0.660000,B=1.000000,A=1.000000)" 3.0)
  (Networking|SwitchHasAuthority
    (:Authority
      (bind _result (Math|Integer|IncrementInt (Variables|Gameplay|GetCurrentPhase))
        (:%20%20
          (for _array_element (.Phaseobjectives (Utilities|Struct|BreakDestructionPhase (Utilities|Array|Get(acopy) (Variables|Gameplay|GetPhases%20setup) (- _result 1))))
            (EventDispatchers|AssignDestructionObjectiveMet _array_element (delegate Custom|PhaseObjectiveMet))
            (switch Utilities|FlowControl|Switch|SwitchonESQTeam (Variables|Gameplay|GetWinningTeamOnLastPhaseComplete)
              (:Team_One
                (Class|SQTeamActor|SetTeam _array_element "Team_Two"))
              (:Team_Two
                (Class|SQTeamActor|SetTeam _array_element "Team_One")))
            (Default|OnShown _array_element (Variables|Gameplay|GetObjective%20class)))
          (Default|CallPhaseStarted (Variables|Gameplay|GetCurrentPhase)))))))

(event Custom|PhaseObjectiveMet
  (params (Objective :type SQ%20Objective%20Object%20Reference))
  (bind _delaybetweenphases (Variables|Gameplay|GetDelayBetweenPhases))
  ;[1 1 1] Handler for phase objective completion
  (Networking|SwitchHasAuthority
    (:Authority
      (Default|CallPhaseObjectiveMet Objective)
      (Default|CallAdjustTicketsforObjective Objective)
      (if (CallFunction|CheckActiveObjectives)
        (Development|PrintString "No active objectives, going to next phase")
        (if (CallFunction|IsCurrentPhaseLast)
          (Development|PrintString "Last phase ended")
          (Default|CallLastPhaseEnded)
          (else
            (Default|CallPhaseEnded (Variables|Gameplay|GetCurrentPhase))
            (bind _returnvalue (Utilities|Time|SetTimerbyFunctionName 0 "Event StartNewPhase" (Math|Conversions|ToFloat(Integer) _delaybetweenphases)))
            (Variables|Default|SetPhaseStartTimer _returnvalue)
            (Development|PrintString (Utilities|String|Append "Starting new phase in " (Utilities|String|ToString(Integer) _delaybetweenphases) " seconds"))
            (bind _returnvalue_2 (Utilities|Time|SetTimerbyFunctionName 0 "Event ShowTimeToPhaseStart" (/ (Math|Conversions|ToFloat(Integer) (Variables|Gameplay|GetDelayBetweenPhases)) 4.0) true))
            (Variables|Default|SetUpdateTimer _returnvalue_2)))
        (else
          (Development|PrintString "Some objectives are still active"))))))

(event Custom|Event%20ShowTimeToPhaseStart
  ;[1 1 1] Send message to the attackers "X seconds left till new orders" (timer value till next phase start)
  (Default|CallSendNotificationtoTeam (Variables|Gameplay|GetWinningTeamOnLastPhaseComplete) (Utilities|String|Append (Utilities|String|ToString(Integer) (Math|Float|Floor (Utilities|Time|GetTimerRemainingTimebyHandle (Variables|Default|GetPhaseStartTimer)))) " seconds left till new orders")))

(event EventBeginPlay
  (Networking|SwitchHasAuthority
    (:Authority
      (Class|SQGameMode|RegisterImportantActor (CallFunction|GetSquadGameMode) self)
      (Variables|Gameplay|SetNumberOfPhases (Utilities|Array|Length (Variables|Gameplay|GetPhases%20setup))))
    (:Remote
      (Utilities|FlowControl|Delay 3.0)
      (CallFunction|GenerateLattice))))

(fn ConstructionScript)

(fn IsCurrentPhaseLast
  (return (== (Variables|Gameplay|GetCurrentPhase) (Variables|Gameplay|GetNumberOfPhases))))

(fn CheckActiveObjectives
  (for _array_element (.Phaseobjectives (Utilities|Struct|BreakDestructionPhase (Utilities|Array|Get(acopy) (Variables|Gameplay|GetPhases%20setup) (- (Variables|Gameplay|GetCurrentPhase) 1))))
    (if (not (Variables|/Script/Squad.SQObjective|GetbHasObjectiveBeenMet _array_element))
      (return false)))
  (return true))

(fn GenerateLattice
  (bind _phaseobjcentroids (LocalVariables|GetPhaseObjCentroids))
  (Development|PrintString "Generate Lattice call")
  (bind _outactors (Actor|GetAllActorsOfClass "/Chora_DES_v1/Gameplay/MapPaint/BP_MapPainter_V2.BP_MapPainter_V2_C"))
  (bind _output_get (LocalVariables|Setmap%20painter%20ref (Utilities|Array|Get(acopy) _outactors)))
  (Utilities|IsValid _output_get
    (:Is%20Valid
      (for _array_element (Variables|Gameplay|GetPhases%20setup)
        (bind _returnvalue (Class|GameplayStatics|GetActorArrayAverageLocation (.Phaseobjectives (Utilities|Struct|BreakDestructionPhase _array_element))))
        (bind _output_get_2 (LocalVariables|SetcurrentCentroid _returnvalue))
        (Utilities|Array|Add (LocalVariables|GetPhaseObjCentroids) _output_get_2)
        (for _array_element_2 (.Phaseobjectives (Utilities|Struct|BreakDestructionPhase _array_element))
          (bind _returnvalue_2 (Game|SpawnActorfromClass "/Chora_DES_v1/Gameplay/MapPaint/BP_DrawedSpline.BP_DrawedSpline_C" (Math|Transform|MakeTransform _output_get_2 "0, 0, 0" "1,1,1") "Undefined" 0 0))
          (Default|ChangeSplineForm _returnvalue_2 (Utilities|Array|MakeArray (LocalVariables|GetcurrentCentroid) (Transformation|GetActorLocation _array_element_2)))
          (Variables|/Chora_DES_v1/Gameplay/MapPaint/BP_DrawedSpline.BP_DrawedSpline_C|SetColoring _returnvalue_2 "(R=1.000000,G=0.352941,B=0.000000,A=1.000000)")
          (Default|AddDrawedSpline (LocalVariables|Getmap%20painter%20ref) _returnvalue_2)))
      (for (_array_element_3 _array_index) _phaseobjcentroids
        (if (not (== _array_index (Utilities|Array|LastIndex _phaseobjcentroids)))
          (bind _returnvalue_3 (Game|SpawnActorfromClass "/Chora_DES_v1/Gameplay/MapPaint/BP_DrawedSpline.BP_DrawedSpline_C" (Math|Transform|MakeTransform _array_element_3 "0, 0, 0" "1,1,1") "Undefined" 0 0))
          (Default|ChangeSplineForm _returnvalue_3 (Utilities|Array|MakeArray _array_element_3 (Utilities|Array|Get(acopy) _phaseobjcentroids (+ _array_index 1))))
          (Variables|/Chora_DES_v1/Gameplay/MapPaint/BP_DrawedSpline.BP_DrawedSpline_C|SetColoring _returnvalue_3 "(R=1.000000,G=0.352941,B=0.000000,A=1.000000)")
          (Default|AddDrawedSpline (LocalVariables|Getmap%20painter%20ref) _returnvalue_3))))
    (:Is%20Not%20Valid
      (Development|PrintString "Can't find MapPainter to draw lattice" true false "(R=0.000000,G=0.660000,B=1.000000,A=1.000000)" 5.0))))