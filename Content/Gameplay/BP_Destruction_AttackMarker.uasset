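; BP_Destruction_AttackMarker is a marker for a possible destruction objective that a team can discover, flagged as the real cache or not.
; On the server, a soldier of the matching team entering its trigger sphere, sized by TriggerDistance, marks it discovered once and fires the Discovered dispatcher.
; ForceDiscoverAsLastMarker silently sets the discovered flag on the real spot.
; The discovery RepNotify is empty; its client map icon update is disconnected.
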(event OnComponentBeginOverlap(Sphere)
  (params (OverlappedComponent :type Primitive%20Component%20Object%20Reference) (OtherActor :type Actor%20Object%20Reference) (OtherComp :type Primitive%20Component%20Object%20Reference) (OtherBodyIndex :type Integer) (bFromSweep :type Boolean) (SweepResult :type Hit%20Result%20Structure%20%28by%20ref%29))
  (Networking|SwitchHasAuthority
    (:Authority
      (bind _assqsoldier (Utilities|Casting|CastToSQSoldier OtherActor))
      (bind _returnvalue (Class|SQSoldier|GetTeam _assqsoldier))
      (if (== (Math|Conversions|ToByte(Integer) _returnvalue) (Variables|Default|GetTeam))
        (CallFunction|Discover)))))

(event EventBeginPlay)

(event Collision|EventActorBeginOverlap
  (params (OtherActor :type Actor%20Object%20Reference)))

(event EventTick
  (params (DeltaSeconds :type Float%20%28single-precision%29)))

(fn ConstructionScript
  (Components|Sphere|SetSphereRadius (Variables|Default|GetSphere) (Variables|Default|GetTriggerDistance) true))

(fn Discover
  (if (not (Variables|Default|GetbIsDiscovered))
    (Variables|Default|SetbIsDiscovered true)
    (Default|CallDiscovered self (Variables|Default|GetReal%20Spot))))

(fn ForceDiscoverasLastMarker
  (if (Variables|Default|GetReal%20Spot)
    (Variables|Default|SetbIsDiscovered true)))

(fn OnRepBIsDiscovered)