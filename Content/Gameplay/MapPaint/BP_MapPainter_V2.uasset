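; Client-side actor that paints registered, colored splines onto the level's map texture from SQWorldSettings.
; Init retries until the map corner actors are valid, derives world units per pixel, and swaps in a runtime render target copy of the map.
; Each tick, and on spline add or remove, it draws splines as line segments into a persistent layer target, then composites that through a material over the original map.
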(event Custom|Redraw
  (bind _spline_render_layer (Variables|Default|GetSpline%20Render%20Layer))
  (bind _mapwidth (Variables|Default|GetMapWidth))
  (bind _mapheight (Variables|Default|GetMapHeight))
  (bind _returnvalue (Math|Conversions|ToFloat(Integer) _mapwidth))
  (bind _returnvalue_2 (Math|Conversions|ToFloat(Integer) _mapheight))
  (bind _returnvalue_3 (Math|Vector2D|MakeVector2D _returnvalue _returnvalue_2))
  (bind (_canvas _size _context) (Rendering|BeginDrawCanvastoRenderTarget _spline_render_layer))
  (Rendering|ClearRenderTarget2D _spline_render_layer)
  (for _array_element (Variables|Default|GetSplineArray)
    (CallFunction|DrawSpline _array_element 0.01 _canvas (Variables|/Chora_DES_v1/Gameplay/MapPaint/BP_DrawedSpline.BP_DrawedSpline_C|GetColoring _array_element) 6.0))
  (Rendering|EndDrawCanvastoRenderTarget _context)
  ;[1 1 1] Drawing map with splines
  (bind (_canvas_2 _size_2 _context_2) (Rendering|BeginDrawCanvastoRenderTarget (Variables|Default|Getedited_map)))
  (Canvas|DrawTexture :self _canvas_2 :RenderTexture (Variables|Default|Getdefault_map) :ScreenSize _returnvalue_3 :BlendMode "BLEND_Opaque" :Rotation 0.0) ; clean map
  (Canvas|DrawMaterial :self _canvas_2 :RenderMaterial "/Chora_DES_v1/Gameplay/MapPaint/mappainter_material.mappainter_material" :ScreenSize _returnvalue_3) ; drawing layer with drawed splines
  (Rendering|EndDrawCanvastoRenderTarget _context_2))

(event Custom|Retry%20Init
  (Utilities|FlowControl|Delay 3.0)
  (Networking|SwitchHasAuthority
    (:Remote
      ;[1 1 1] dynamic map init
      (bind _returnvalue (Class|SQBlueprintLibrary|GetWorldSettings))
      (bind _assqworld_settings (Utilities|Casting|CastToSQWorldSettings _returnvalue)
        (:then
          (Variables|Default|Setworldsettings _assqworld_settings)
          (bind _output_get (Variables|Default|Setdefault_map (Variables|/Script/Squad.SQWorldSettings|GetMapTexture _assqworld_settings)))
          (Utilities|IsValid (Variables|/Script/Squad.SQWorldSettings|GetMapTextureCornerZero _assqworld_settings)
            (:Is%20Valid
              (Utilities|IsValid (Variables|/Script/Squad.SQWorldSettings|GetMapTextureCornerOne _assqworld_settings)
                (:Is%20Valid
                  (bind _astexture_2d (Utilities|Casting|CastToTexture2D _output_get))
                  (bind _output_get_2 (Variables|Default|SetMapWidth (Class|Texture2D|BlueprintGetSizeX _astexture_2d)))
                  (bind _output_get_3 (Variables|Default|SetMapHeight (Class|Texture2D|BlueprintGetSizeY _astexture_2d)))
                  (bind (_unitsperpixelx _unitsperpixely) (CallFunction|GetUnitsPerPixel _output_get_2 _output_get_3 (Transformation|GetActorLocation (Variables|/Script/Squad.SQWorldSettings|GetMapTextureCornerZero _assqworld_settings)) (Transformation|GetActorLocation (Variables|/Script/Squad.SQWorldSettings|GetMapTextureCornerOne _assqworld_settings))))
                  (Variables|Default|SetUnitPerPixelX _unitsperpixelx)
                  (Variables|Default|SetUnitsPerPixelY _unitsperpixely)
                  (bind _returnvalue_2 (Rendering|CreateRenderTarget2D _output_get_2 _output_get_3))
                  (bind _output_get_4 (Variables|Default|Setedited_map _returnvalue_2))
                  (bind (_canvas _size _context) (Rendering|BeginDrawCanvastoRenderTarget _output_get_4))
                  (Canvas|DrawTexture :self _canvas :RenderTexture (Variables|Default|Getdefault_map) :BlendMode "BLEND_Opaque")
                  (Rendering|EndDrawCanvastoRenderTarget _context)
                  (Variables|/Script/Squad.SQWorldSettings|SetMapTexture (Variables|Default|Getworldsettings) (Variables|Default|Getedited_map))
                  (Class|SQBlueprintLibrary|SetTextureRenderTarget2DSize (Variables|Default|GetSpline%20Render%20Layer) (Variables|Default|GetMapWidth) (Variables|Default|GetMapHeight))
                  (Variables|Default|SetInitialized true))
                (:Is%20Not%20Valid
                  (CallFunction|RetryInit :!label _label))))
            (:Is%20Not%20Valid
              (goto _label))))
        (:CastFailed
          (CallFunction|RetryInit))))))

(event EventBeginPlay
  (Networking|SwitchHasAuthority
    (:Remote
      ;[1 1 1] dynamic map init
      (bind _returnvalue (Class|SQBlueprintLibrary|GetWorldSettings))
      (bind _assqworld_settings (Utilities|Casting|CastToSQWorldSettings _returnvalue)
        (:then
          (Variables|Default|Setworldsettings _assqworld_settings)
          (bind _output_get (Variables|Default|Setdefault_map (Variables|/Script/Squad.SQWorldSettings|GetMapTexture _assqworld_settings)))
          (Utilities|IsValid (Variables|/Script/Squad.SQWorldSettings|GetMapTextureCornerZero _assqworld_settings)
            (:Is%20Valid
              (Utilities|IsValid (Variables|/Script/Squad.SQWorldSettings|GetMapTextureCornerOne _assqworld_settings)
                (:Is%20Valid
                  (bind _astexture_2d (Utilities|Casting|CastToTexture2D _output_get))
                  (bind _output_get_2 (Variables|Default|SetMapWidth (Class|Texture2D|BlueprintGetSizeX _astexture_2d)))
                  (bind _output_get_3 (Variables|Default|SetMapHeight (Class|Texture2D|BlueprintGetSizeY _astexture_2d)))
                  (bind (_unitsperpixelx _unitsperpixely) (CallFunction|GetUnitsPerPixel _output_get_2 _output_get_3 (Transformation|GetActorLocation (Variables|/Script/Squad.SQWorldSettings|GetMapTextureCornerZero _assqworld_settings)) (Transformation|GetActorLocation (Variables|/Script/Squad.SQWorldSettings|GetMapTextureCornerOne _assqworld_settings))))
                  (Variables|Default|SetUnitPerPixelX _unitsperpixelx)
                  (Variables|Default|SetUnitsPerPixelY _unitsperpixely)
                  (bind _returnvalue_2 (Rendering|CreateRenderTarget2D _output_get_2 _output_get_3))
                  (bind _output_get_4 (Variables|Default|Setedited_map _returnvalue_2))
                  (bind (_canvas _size _context) (Rendering|BeginDrawCanvastoRenderTarget _output_get_4))
                  (Canvas|DrawTexture :self _canvas :RenderTexture (Variables|Default|Getdefault_map) :BlendMode "BLEND_Opaque")
                  (Rendering|EndDrawCanvastoRenderTarget _context)
                  (Variables|/Script/Squad.SQWorldSettings|SetMapTexture (Variables|Default|Getworldsettings) (Variables|Default|Getedited_map))
                  (Class|SQBlueprintLibrary|SetTextureRenderTarget2DSize (Variables|Default|GetSpline%20Render%20Layer) (Variables|Default|GetMapWidth) (Variables|Default|GetMapHeight))
                  (Variables|Default|SetInitialized true))
                (:Is%20Not%20Valid
                  (CallFunction|RetryInit :!label _label))))
            (:Is%20Not%20Valid
              (goto _label))))
        (:CastFailed
          (CallFunction|RetryInit))))))

(event Collision|EventActorBeginOverlap
  (params (OtherActor :type Actor%20Object%20Reference)))

(event EventTick
  (params (DeltaSeconds :type Float%20%28single-precision%29))
  (bind _edited_map (Variables|Default|Getedited_map))
  (bind _worldsettings (Variables|Default|Getworldsettings))
  (Networking|SwitchHasAuthority
    (:Remote
      (if (Variables|Default|GetInitialized)
        (if (== _edited_map (Variables|/Script/Squad.SQWorldSettings|GetMapTexture _worldsettings))
          _
          (else
            (Variables|/Script/Squad.SQWorldSettings|SetMapTexture _worldsettings _edited_map)))
        (CallFunction|Redraw)))))

(fn ConstructionScript)

(fn GetUnitsPerPixel
  (params (Map%20Width :type Integer) (Map%20Height :type Integer) (Map%20Corner%20Zero :type Vector) (Map%20Corner%20One :type Vector))
  (bind (_x _y) (Math|Vector|BreakVector Map%20Corner%20Zero))
  (bind (_x_2 _y_2) (Math|Vector|BreakVector Map%20Corner%20One))
  (if (< (.X (Math|Vector|BreakVector Map%20Corner%20Zero)) (.X (Math|Vector|BreakVector Map%20Corner%20One)))
    (Variables|Default|SetMapCornerLeft Map%20Corner%20Zero)
    (Variables|Default|SetMapCornerRight Map%20Corner%20One)
    (else
      (Variables|Default|SetMapCornerLeft Map%20Corner%20One)
      (Variables|Default|SetMapCornerRight Map%20Corner%20Zero)))
  ;[1 1 1] Вычисление северо-западного угла на карте (Х растет на восток, Y растет на юг)
  (if (< (.Y (Math|Vector|BreakVector (Variables|Default|GetMapCornerLeft))) (.Y (Math|Vector|BreakVector (Variables|Default|GetMapCornerRight))))
    _
    (else
      (Variables|Default|SetMapCornerLeft (Math|Vector|MakeVector (.X (Math|Vector|BreakVector (Variables|Default|GetMapCornerLeft))) (.Y (Math|Vector|BreakVector (Variables|Default|GetMapCornerRight))) (.Z (Math|Vector|BreakVector (Variables|Default|GetMapCornerLeft)))))))
  (return (/ (Math|Float|Absolute(Float) (- _x _x_2)) (Math|Conversions|ToFloat(Integer) Map%20Width)) (/ (Math|Float|Absolute(Float) (- _y _y_2)) (Math|Conversions|ToFloat(Integer) Map%20Height))))

(fn LocationtoScreenCoords
  (params (Location :type Vector))
  (bind _mapcornerleft (Variables|Default|GetMapCornerLeft))
  (bind (_x _y) (Math|Vector|BreakVector _mapcornerleft))
  (bind _output_get (LocalVariables|SetLoc Location))
  (LocalVariables|SetX (/ (Math|Float|Absolute(Float) (- _x (.X (Math|Vector|BreakVector _output_get)))) (Variables|Default|GetUnitPerPixelX)))
  (LocalVariables|SetY (/ (Math|Float|Absolute(Float) (- _y (.Y (Math|Vector|BreakVector _output_get)))) (Variables|Default|GetUnitsPerPixelY)))
  (return (Math|Vector2D|MakeVector2D (LocalVariables|GetX) (LocalVariables|GetY))))

(fn DrawSpline
  (params (Spline%20to%20Draw :type BP%20Drawed%20Spline%20Object%20Reference) (Resolution :type Float%20%28single-precision%29) (Canvas :type Canvas%20Object%20Reference) (Color :type Linear%20Color%20Structure) (Thickness :type Float%20%28single-precision%29))
  (bind _unitperpixelx (Variables|Default|GetUnitPerPixelX))
  (bind _unitsperpixely (Variables|Default|GetUnitsPerPixelY))
  (bind _returnvalue (Math|Float|Min(Float) _unitperpixelx _unitsperpixely))
  (LocalVariables|SetCanvas%20Ref Canvas)
  (LocalVariables|SetRender%20Thickness Thickness)
  (LocalVariables|SetRenderColor Color)
  (bind _output_get (LocalVariables|SetSplineRef (Variables|/Chora_DES_v1/Gameplay/MapPaint/BP_DrawedSpline.BP_DrawedSpline_C|GetSpline Spline%20to%20Draw)))
  (bind _output_get_2 (LocalVariables|SetStep (Math|Float|Lerp 0.0 (Spline|GetSplineLength _output_get) Resolution)))
  (if (< (LocalVariables|GetStep) _returnvalue)
    (LocalVariables|SetStep _returnvalue))
  (LocalVariables|SetNextDistance (+ _output_get_2 (LocalVariables|GetCurrentDistance)))
  (while (< (LocalVariables|GetNextDistance) (Spline|GetSplineLength _output_get))
    (Class|Canvas|DrawLine (LocalVariables|GetCanvas%20Ref) (CallFunction|LocationtoScreenCoords (Spline|GetLocationatDistanceAlongSpline (LocalVariables|GetSplineRef) (LocalVariables|GetCurrentDistance) "World")) (CallFunction|LocationtoScreenCoords (Spline|GetLocationatDistanceAlongSpline (LocalVariables|GetSplineRef) (LocalVariables|GetNextDistance) "World")) (LocalVariables|GetRender%20Thickness) (LocalVariables|GetRenderColor))
    (LocalVariables|SetCurrentDistance (LocalVariables|GetNextDistance))
    (LocalVariables|SetNextDistance (+ (LocalVariables|GetNextDistance) (LocalVariables|GetStep))))
  (Class|Canvas|DrawLine (LocalVariables|GetCanvas%20Ref) (CallFunction|LocationtoScreenCoords (Spline|GetLocationatDistanceAlongSpline (LocalVariables|GetSplineRef) (LocalVariables|GetCurrentDistance) "World")) (CallFunction|LocationtoScreenCoords (Spline|GetLocationatDistanceAlongSpline (LocalVariables|GetSplineRef) (Spline|GetSplineLength _output_get) "World")) (LocalVariables|GetRender%20Thickness) (LocalVariables|GetRenderColor)))

(fn AddDrawedSpline
  (params (Spline :type BP%20Drawed%20Spline%20Object%20Reference))
  (Utilities|Array|AddUnique (Variables|Default|GetSplineArray) Spline)
  (CallFunction|Redraw))

(fn RemoveDrawedSpline
  (params (Spline :type BP%20Drawed%20Spline%20Object%20Reference))
  (Utilities|Array|RemoveItem (Variables|Default|GetSplineArray) Spline)
  (CallFunction|Redraw))