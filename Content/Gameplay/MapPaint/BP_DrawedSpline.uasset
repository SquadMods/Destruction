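; Spline actor in the MapPaint folder that holds a drawn path, with a shape that can be replaced at runtime.
; ChangeSplineForm clears the spline and rebuilds it from an array of world-space points.
; UpdateIsLinear sets an IsLinear flag, true only when every spline point is Linear, and runs on construction and after each rebuild.
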(event EventBeginPlay)

(event Collision|EventActorBeginOverlap
  (params (OtherActor :type Actor%20Object%20Reference)))

(event EventTick
  (params (DeltaSeconds :type Float%20%28single-precision%29)))

(fn ConstructionScript
  (CallFunction|UpdateIsLinear))

(fn ChangeSplineForm
  (params (Points :type Array%20of%20Vectors))
  (bind _spline (Variables|Default|GetSpline))
  (Spline|ClearSplinePoints _spline true)
  (for _array_element Points
    (Spline|AddSplinePoint _spline _array_element "World" true))
  (CallFunction|UpdateIsLinear))

(fn UpdateIsLinear
  (bind _spline (Variables|Default|GetSpline))
  (for _index (range 0 (- (Spline|GetNumberOfSplinePoints _spline) 1))
    (if (not (Utilities|Enum|Equal(Enum) (Class|SplineComponent|GetSplinePointType _spline _index) "Linear"))
      (Variables|Default|SetisLinear false)
      (return)))
  (Variables|Default|SetisLinear true))