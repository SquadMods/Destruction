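; Ruleset for the Squad Destruction game mode, pitting attackers against defenders over phased objectives and delegating phase logic to a registered BP_DestructionPhaseDirector.
; On registration it derives team roles from the director's last-phase winner, sets per-team rules, defaults victory to defenders and binds director events.
; The server starts the first phase after a delay.
; Director events drive team chat notifications, objective ticket adjustments and match end, when the last-phase winner takes victory.
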(event Custom|Event%20Objective%20Destroyed
  (params (Objective :type SQ%20Objective%20Object%20Reference))
  (Class|SQGameRuleSet|SendChatMessage "GameNotificationTeam" (Utilities|String|ToString(Text) (Variables|/Script/Squad.SQObjective|GetObjectiveMetOwningTeamMessage Objective)) (Variables|Default|GetDefendersTeam) 0 false)
  (Class|SQGameRuleSet|SendChatMessage "GameNotificationTeam" (Utilities|String|ToString(Text) (Variables|/Script/Squad.SQObjective|GetObjectiveMetOpposingTeamMessage Objective)) (Variables|Default|GetAttackersTeam) 0 false))

(event Custom|FinishRound
  (Variables|Default|SetisReadyToEndMatch true))

(event Custom|PhaseStartedMessage
  (params (Phase%20Number :type Integer))
  (Class|SQGameRuleSet|SendChatMessage "GameNotificationTeam" (Variables|Default|GetDefenders%20message%20on%20Phase%20Start) (Variables|Default|GetDefendersTeam) 0 false)
  (Class|SQGameRuleSet|SendChatMessage "GameNotificationTeam" (Variables|Default|GetAttackers%20message%20on%20Phase%20Start) (Variables|Default|GetAttackersTeam) 0 false))

(event Custom|PhaseEndedMessage
  (params (Phase%20Number :type Integer))
  (Class|SQGameRuleSet|SendChatMessage "GameNotificationTeam" (Variables|Default|GetDefenders%20message%20on%20Phase%20End) (Variables|Default|GetDefendersTeam) 0 false)
  (Class|SQGameRuleSet|SendChatMessage "GameNotificationTeam" (Variables|Default|GetAttackers%20message%20on%20Phase%20End) (Variables|Default|GetAttackersTeam) 0 false))

(event Custom|Event%20Adjust%20Tickets%20for%20Objective
  (params (Objective :type SQ%20Objective%20Object%20Reference))
  (CallFunction|AdjustTicketsforObjectiveMet Objective))

(event EventMatchStarted
  (bind _phasedirector (Variables|Default|GetPhaseDirector))
  (Networking|SwitchHasAuthority
    (:Authority
      (Utilities|IsValid _phasedirector
        (:Is%20Valid
          (Utilities|FlowControl|Delay 1e+01)
          (Development|PrintString "Starting game mode logic" false true "(R=0.000000,G=0.660000,B=1.000000,A=1.000000)" 5.0)
          (Default|EventStartNewPhase _phasedirector))))))

(event EventRegisterActor
  (params (actor :type Actor%20Object%20Reference))
  ;[1 1 1] Registering reference to Phase Director, who does all the work
  (bind _asbp_destruction_phase_director (Utilities|Casting|CastToBP_DestructionPhaseDirector actor))
  (bind _output_get (Variables|Default|SetPhaseDirector _asbp_destruction_phase_director))
  (CallFunction|SetupShownRulesforTeams)
  (EventDispatchers|BindEventtoLastPhaseEnded _output_get (delegate Custom|FinishRound))
  (EventDispatchers|BindEventtoAdjustTicketsforObjective _output_get (delegate Custom|Event%20Adjust%20Tickets%20for%20Objective))
  (EventDispatchers|BindEventtoPhaseObjectiveMet _output_get (delegate Custom|Event%20Objective%20Destroyed))
  (EventDispatchers|BindEventtoPhaseStarted _output_get (delegate Custom|PhaseStartedMessage))
  (EventDispatchers|BindEventtoPhaseEnded _output_get (delegate Custom|PhaseEndedMessage)))

(event EventBeginPlay
  (Utilities|FlowControl|Delay 5.0)
  (Utilities|IsValid (stale EventRegisterActor _output_get)
    (:Is%20Not%20Valid
      (Development|PrintString "Not found phase director! Game mode will be non-functional"))))

(event EventUnregisterActor
  (params (actor :type Actor%20Object%20Reference))
  ;[1 1 1] Registering reference to Phase Director, who does all the work
  (Utilities|Casting|CastToBP_DestructionPhaseDirector actor)
  (Variables|Default|SetPhaseDirector 0))

(fn ConstructionScript)

(fn ReadytoEndMatch
  (if (Variables|Default|GetisReadyToEndMatch)
    (Class|SQGameModeRuleset|SetWinningTeamfromEnum (Variables|/Chora_DES_v1/Gameplay/BP_DestructionPhaseDirector.BP_DestructionPhaseDirector_C|GetWinningTeamOnLastPhaseComplete (Variables|Default|GetPhaseDirector)))
    (return "ReadyToEndMatch")
    (else
      (return "Unhandled"))))

(fn AdjustTicketsforObjectiveMet
  (params (Objective%20met :type SQ%20Objective%20Object%20Reference))
  (bind _returnvalue (Class|SQTeamActor|GetTeam Objective%20met))
  (LocalVariables|SetObjective Objective%20met)
  (switch Utilities|FlowControl|Switch|SwitchonESQTeam _returnvalue
    (:Team_Neutral
      (return))
    (:Team_One
      (LocalVariables|SetOpposing%20Team "Team_Two"))
    (:Team_Two
      (LocalVariables|SetOpposing%20Team "Team_One")))
  (LocalVariables|SetOwning%20Team _returnvalue)
  (CallFunction|AdjustTeamTickets (LocalVariables|GetOwning%20Team) (Variables|/Script/Squad.SQObjective|GetTicketAdjustmentByOwningTeamUponObjectiveBeingMet (LocalVariables|GetObjective)))
  (CallFunction|AdjustTeamTickets (LocalVariables|GetOpposing%20Team) (Variables|/Script/Squad.SQObjective|GetTicketAdjustmentByOpposingTeamUponObjectiveBeingMet (LocalVariables|GetObjective))))

(fn AdjustTeamTickets
  (params (Team :type ESQTeam%20Enum) (by%20Amount :type Integer))
  (bind _return_value (CallFunction|GetSquadGameMode))
  (bind _returnvalue (Class|SQGameMode|GetTeam _return_value Team))
  (bind _teamstate (Variables|/Script/Squad.SQTeam|GetTeamState _returnvalue))
  (Variables|/Script/Squad.SQTeamState|SetTickets _teamstate (+ (Variables|/Script/Squad.SQTeamState|GetTickets _teamstate) by%20Amount)))

(fn SetupShownRulesforTeams
  (bind _rulestobeshownwhenplayersjoinateam (Variables|Default|GetRulesToBeShownWhenPlayersJoinATeam))
  (switch Utilities|FlowControl|Switch|SwitchonESQTeam (Variables|/Chora_DES_v1/Gameplay/BP_DestructionPhaseDirector.BP_DestructionPhaseDirector_C|GetWinningTeamOnLastPhaseComplete (Variables|Default|GetPhaseDirector))
    (:Team_One
      (Variables|Default|SetAttackersTeam "Team_One")
      (Variables|Default|SetDefendersTeam "Team_Two"))
    (:Team_Two
      (Variables|Default|SetAttackersTeam "Team_Two")
      (Variables|Default|SetDefendersTeam "Team_One")))
  (Utilities|Array|Add _rulestobeshownwhenplayersjoinateam (Utilities|Struct|MakeSQGameModeRules (Variables|Default|GetAttackersTeam) (Variables|Default|GetRulesForAttackers)))
  (Utilities|Array|Add _rulestobeshownwhenplayersjoinateam (Utilities|Struct|MakeSQGameModeRules (Variables|Default|GetDefendersTeam) (Variables|Default|GetRulesForDefenders)))
  (Class|SQGameModeRuleset|SetWinningTeamfromEnum (Variables|Default|GetDefendersTeam)) ; Set Defenders to win by default
)