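; US FOB radio deployable that adds team-specific no-deploy zone checks to the placement rules it inherits.
; BPExtraPlacementRules scans the StackingCollisionBox for overlapping BP_NoDeployZone_Custom actors and rejects placement with a DEPLOYZONE reason if one disallows the neutral team or the radio's team.
; Otherwise the parent rules decide the result.
; The event graph and construction script add no logic.
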(event EventBeginPlay)

(event Collision|EventActorBeginOverlap
  (params (OtherActor :type Actor%20Object%20Reference)))

(event EventTick
  (params (DeltaSeconds :type Float%20%28single-precision%29)))

(fn ConstructionScript)

(fn BPExtraPlacementRules
  (bind _stackingcollisionbox (Variables|Default|GetStackingCollisionBox))
  (bind _overlappingactors (Collision|GetOverlappingActors _stackingcollisionbox "/Chora_DES_v1/Gameplay/BP_NoDeployZone_Custom.BP_NoDeployZone_Custom_C" :!class /Script/Engine.PrimitiveComponent))
  (if (> (Utilities|Array|Length _overlappingactors) 0)
    (for _array_element _overlappingactors
      (bind _asbp_no_deploy_zone_custom (Utilities|Casting|CastToBP_NoDeployZone_Custom _array_element))
      (if (or (Utilities|Enum|Equal(Enum) (Variables|/Chora_DES_v1/Gameplay/BP_NoDeployZone_Custom.BP_NoDeployZone_Custom_C|GetDisallowed%20Team _asbp_no_deploy_zone_custom) "Team_Neutral") (== (Variables|/Chora_DES_v1/Gameplay/BP_NoDeployZone_Custom.BP_NoDeployZone_Custom_C|GetDisallowed%20Team _asbp_no_deploy_zone_custom) (Math|Conversions|ToByte(Integer) (Variables|Default|GetTeam))))
        (return "NO_DEPLOY_ZONE" false))))
  (bind (_reason _returnvalue) (|CallParentFunction))
  (return _reason _returnvalue))